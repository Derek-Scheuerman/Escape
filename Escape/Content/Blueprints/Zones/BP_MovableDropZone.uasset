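; BP_MovableDropZone is a trigger zone that rewards the player when a BP_Movable object is moved into its DropZone component.
; On overlap it has the movable add either the current room key or a named item to the player's inventory, with the room key taking priority.
; An AddedItem flag is set after a grant so the zone pays out only once.
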(event OnComponentBeginOverlap(DropZone)
  (params (OverlappedComponent :type Primitive%20Component%20Object%20Reference) (OtherActor :type Actor%20Object%20Reference) (OtherComp :type Primitive%20Component%20Object%20Reference) (OtherBodyIndex :type Integer) (bFromSweep :type Boolean) (SweepResult :type Hit%20Result%20Structure%20%28by%20ref%29))
  (if (not (Variables|Default|GetAddedItem))
    (bind _asbp_movable (Utilities|Casting|CastToBP_Movable OtherActor))
    (if (Variables|Default|GetAddRoomKey)
      (Default|AddCurrentRoomKeytoPlayerInv _asbp_movable)
      (Variables|Default|SetAddedItem true)
      (elif (Variables|Default|GetAddItem)
        (Default|AddItemtoPlayerInv _asbp_movable (Variables|Default|GetItemName))
        (Variables|Default|SetAddedItem true)))))

(event EventBeginPlay)

(event Collision|EventActorBeginOverlap
  (params (OtherActor :type Actor%20Object%20Reference)))

(event EventTick
  (params (DeltaSeconds :type Float%20%28single-precision%29)))

(fn ConstructionScript)