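; Ball maze puzzle where left and right pressure plates move maze pieces to guide a ball to the exit.
; Overlaps play and reverse two timelines that offset from cached start positions: left drives boxes and a tilt piece, right drives a wall, each sinking its button.
; Table or reset-trigger overlaps teleport the ball back to start.
; Reaching the end once adds a configurable reward to the first-person character's inventory.
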(event OnComponentBeginOverlap(Reset_Collision)
  (params (OverlappedComponent :type Primitive%20Component%20Object%20Reference) (OtherActor :type Actor%20Object%20Reference) (OtherComp :type Primitive%20Component%20Object%20Reference) (OtherBodyIndex :type Integer) (bFromSweep :type Boolean) (SweepResult :type Hit%20Result%20Structure%20%28by%20ref%29))
  ;[0.15 0.15 0.15 0.5] Reset Ball Location
  (Transformation|SetRelativeTransform (Variables|Default|GetPlayBall) (Variables|Default|GetPlayBallStartLocation) false true))

(event OnComponentBeginOverlap(Box)
  (params (OverlappedComponent :type Primitive%20Component%20Object%20Reference) (OtherActor :type Actor%20Object%20Reference) (OtherComp :type Primitive%20Component%20Object%20Reference) (OtherBodyIndex :type Integer) (bFromSweep :type Boolean) (SweepResult :type Hit%20Result%20Structure%20%28by%20ref%29))
  ;[0.15 0.15 0.15 0.5] Ball hit table, Reset ball
  (if (== OtherComp (Variables|Default|GetPlayBall))
    (Transformation|SetRelativeTransform (Variables|Default|GetPlayBall) (Variables|Default|GetPlayBallStartLocation) false true)))

(event OnComponentBeginOverlap(RCollision)
  (params (OverlappedComponent :type Primitive%20Component%20Object%20Reference) (OtherActor :type Actor%20Object%20Reference) (OtherComp :type Primitive%20Component%20Object%20Reference) (OtherBodyIndex :type Integer) (bFromSweep :type Boolean) (SweepResult :type Hit%20Result%20Structure%20%28by%20ref%29))
  (bind _wall1 (Variables|Default|GetWall1))
  (bind _relativelocation (Variables|/Script/Engine.SceneComponent|GetRelativeLocation _wall1))
  ;[0.15 0.15 0.15 0.5] OnBox/OffBox
  ;[0.15 0.15 0.15 0.5] Is the Timeline already Going? Yes? Wait... No? Continue
  (if (Variables|Default|GetOGLocation)
    _
    (else
      (CallFunction|SetAllLocation)
      (Variables|Default|SetOGLocation true)))
  (if (Variables|Default|GetTopTimeLineRunning)
    ;[0.15 0.15 0.15 0.5] Activate Timeline
    (bind (_direction _down _rbuttondown _wall1down) (Timeline|Down Play)
      (:Update
        (Variables|Default|SetBottomTimeLineRunning true)
        (Transformation|SetRelativeLocation (Variables|Default|GetRPressure_Button) (Math|Vector|MakeVector 0.0 0.0 (+ _rbuttondown (Variables|Default|GetRelative%20Location%20Z_1))) false false)
        (Utilities|FlowControl|Sequence
          (:then_0)
          (:then_1
            ;[0.15 0.15 0.15 0.5] Wall1 Down/NoUp
            (Transformation|SetRelativeLocation (Variables|Default|GetWall1) (Math|Vector|MakeVector (.x _relativelocation) (.y _relativelocation) (+ (Variables|Default|GetWall1StartLocation) _wall1down)) false false))))
      (:Finished
        (Variables|Default|SetBottomTimeLineRunning false)))
    (else
      (Timeline|Down Play))))

(event OnComponentEndOverlap(RCollision)
  (params (OverlappedComponent :type Primitive%20Component%20Object%20Reference) (OtherActor :type Actor%20Object%20Reference) (OtherComp :type Primitive%20Component%20Object%20Reference) (OtherBodyIndex :type Integer))
  (bind _wall1 (Variables|Default|GetWall1))
  (bind _relativelocation (Variables|/Script/Engine.SceneComponent|GetRelativeLocation _wall1))
  ;[0.15 0.15 0.15 0.5] OnBox/OffBox
  ;[0.15 0.15 0.15 0.5] Is the Timeline already Going? Yes? Wait... No? Continue
  (if (Variables|Default|GetTopTimeLineRunning)
    ;[0.15 0.15 0.15 0.5] Activate Timeline
    (bind (_direction _down _rbuttondown _wall1down) (Timeline|Down Reverse)
      (:Update
        (Variables|Default|SetBottomTimeLineRunning true)
        (Transformation|SetRelativeLocation (Variables|Default|GetRPressure_Button) (Math|Vector|MakeVector 0.0 0.0 (+ _rbuttondown (Variables|Default|GetRelative%20Location%20Z_1))) false false)
        (Utilities|FlowControl|Sequence
          (:then_0)
          (:then_1
            ;[0.15 0.15 0.15 0.5] Wall1 Down/NoUp
            (Transformation|SetRelativeLocation (Variables|Default|GetWall1) (Math|Vector|MakeVector (.x _relativelocation) (.y _relativelocation) (+ (Variables|Default|GetWall1StartLocation) _wall1down)) false false))))
      (:Finished
        (Variables|Default|SetBottomTimeLineRunning false)))
    (else
      (Timeline|Down Reverse))))

(event OnComponentBeginOverlap(LCollision)
  (params (OverlappedComponent :type Primitive%20Component%20Object%20Reference) (OtherActor :type Actor%20Object%20Reference) (OtherComp :type Primitive%20Component%20Object%20Reference) (OtherBodyIndex :type Integer) (bFromSweep :type Boolean) (SweepResult :type Hit%20Result%20Structure%20%28by%20ref%29))
  (bind _tilt (Variables|Default|GetTilt))
  (bind _test (Variables|Default|GetTEst))
  (bind _relativelocation (Variables|/Script/Engine.SceneComponent|GetRelativeLocation _tilt))
  (bind _relativelocation_2 (Variables|/Script/Engine.SceneComponent|GetRelativeLocation _test))
  ;[0.15 0.15 0.15 0.5] OnBox/OffBox
  ;[0.15 0.15 0.15 0.5] Is the Timeline already going? Yes? Wait... No? Continue
  (if (Variables|Default|GetOGLocation)
    _
    (else
      (CallFunction|SetAllLocation)
      (Variables|Default|SetOGLocation true)))
  (if (Variables|Default|GetBottomTimeLineRunning)
    ;[0.15 0.15 0.15 0.5] Activate Timeline
    (bind (_direction _up _lbuttondown _tiltleft) (Timeline|UP Play)
      (:Update
        (Variables|Default|SetTopTimeLineRunning true)
        (Transformation|SetRelativeLocation (Variables|Default|GetPressure_Button) (Math|Vector|MakeVector 0.0 0.0 (+ _lbuttondown (Variables|Default|GetRelative%20Location%20Z_0))) false false)
        (Utilities|FlowControl|Sequence
          (:then_0
            ;[0.15 0.15 0.15 0.5] Move Boxes Up/Down
            (Transformation|SetRelativeLocation (Variables|Default|GetTEst) (Math|Vector|MakeVector (.x _relativelocation_2) (.y _relativelocation_2) (+ (Variables|Default|GetRelative%20Location%20Z) _up)) false false))
          (:then_1
            ;[0.15 0.15 0.15 0.5] TiltTable Left
            (Transformation|SetRelativeLocation _tilt (Math|Vector|MakeVector (+ _tiltleft (Variables|Default|GetRelative%20Location%20X)) (.y _relativelocation) (.z _relativelocation)) false false))))
      (:Finished
        (Variables|Default|SetTopTimeLineRunning false)))
    (else
      (Timeline|UP Play))))

(event OnComponentEndOverlap(LCollision)
  (params (OverlappedComponent :type Primitive%20Component%20Object%20Reference) (OtherActor :type Actor%20Object%20Reference) (OtherComp :type Primitive%20Component%20Object%20Reference) (OtherBodyIndex :type Integer))
  (bind _tilt (Variables|Default|GetTilt))
  (bind _test (Variables|Default|GetTEst))
  (bind _relativelocation (Variables|/Script/Engine.SceneComponent|GetRelativeLocation _tilt))
  (bind _relativelocation_2 (Variables|/Script/Engine.SceneComponent|GetRelativeLocation _test))
  ;[0.15 0.15 0.15 0.5] OnBox/OffBox
  ;[0.15 0.15 0.15 0.5] Is the Timeline already going? Yes? Wait... No? Continue
  (if (Variables|Default|GetBottomTimeLineRunning)
    ;[0.15 0.15 0.15 0.5] Activate Timeline
    (bind (_direction _up _lbuttondown _tiltleft) (Timeline|UP Reverse)
      (:Update
        (Variables|Default|SetTopTimeLineRunning true)
        (Transformation|SetRelativeLocation (Variables|Default|GetPressure_Button) (Math|Vector|MakeVector 0.0 0.0 (+ _lbuttondown (Variables|Default|GetRelative%20Location%20Z_0))) false false)
        (Utilities|FlowControl|Sequence
          (:then_0
            ;[0.15 0.15 0.15 0.5] Move Boxes Up/Down
            (Transformation|SetRelativeLocation (Variables|Default|GetTEst) (Math|Vector|MakeVector (.x _relativelocation_2) (.y _relativelocation_2) (+ (Variables|Default|GetRelative%20Location%20Z) _up)) false false))
          (:then_1
            ;[0.15 0.15 0.15 0.5] TiltTable Left
            (Transformation|SetRelativeLocation _tilt (Math|Vector|MakeVector (+ _tiltleft (Variables|Default|GetRelative%20Location%20X)) (.y _relativelocation) (.z _relativelocation)) false false))))
      (:Finished
        (Variables|Default|SetTopTimeLineRunning false)))
    (else
      (Timeline|UP Reverse))))

(event OnComponentBeginOverlap(EndCollision)
  (params (OverlappedComponent :type Primitive%20Component%20Object%20Reference) (OtherActor :type Actor%20Object%20Reference) (OtherComp :type Primitive%20Component%20Object%20Reference) (OtherBodyIndex :type Integer) (bFromSweep :type Boolean) (SweepResult :type Hit%20Result%20Structure%20%28by%20ref%29))
  (if (== OtherComp (Variables|Default|GetPlayBall))
    (Utilities|FlowControl|DoOnce false
      (:Completed
        (Development|PrintString "Finished Maze" true true "(R=0.000000,G=0.660000,B=1.000000,A=1.000000)" 1e+01)
        (bind _asbp_first_person_character (Utilities|Casting|CastToBP_FirstPersonCharacter (Game|GetPlayerCharacter 0)))
        (Default|AddtoInv (Variables|/Game/FirstPerson/Blueprints/BP_FirstPersonCharacter.BP_FirstPersonCharacter_C|GetInventorySystem _asbp_first_person_character) (Variables|Default|GetReward) (Variables|Default|GetRewardQuantity))))))

(event EventBeginPlay
  (Variables|Default|SetPlayBallStartLocation (Transformation|GetRelativeTransform (Variables|Default|GetPlayBall))))

(fn ConstructionScript)

(fn SetAllLocation
  (Variables|Default|SetRelative%20Location%20Z (.z (Variables|/Script/Engine.SceneComponent|GetRelativeLocation (Variables|Default|GetTEst))))
  (Variables|Default|SetRelative%20Location%20Z (.z (Variables|/Script/Engine.SceneComponent|GetRelativeLocation (Variables|Default|GetTEst))))
  (Variables|Default|SetRelative%20Location%20Z_0 (.z (Variables|/Script/Engine.SceneComponent|GetRelativeLocation (Variables|Default|GetPressure_Button))))
  (Variables|Default|SetRelative%20Location%20Z_1 (.z (Variables|/Script/Engine.SceneComponent|GetRelativeLocation (Variables|Default|GetRPressure_Button))))
  (Variables|Default|SetWall1StartLocation (.z (Variables|/Script/Engine.SceneComponent|GetRelativeLocation (Variables|Default|GetWall1))))
  (Variables|Default|SetRelative%20Location%20X (.x (Variables|/Script/Engine.SceneComponent|GetRelativeLocation (Variables|Default|GetTilt))))
  (return))