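; BP_Door is an interactable locked door that swings open when the interacting player carries the matching key.
; CheckKey scans the player's InventorySystem contents for the key's item ID; success opens the door with a sound, failure plays a different sound.
; A timeline rotates the DoorPIV pivot by 90 degrees, reversing to close without a key check, while IsRotating blocks re-triggering.
; LookAt builds an "Open {item}" prompt from the door's data table row.
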(event EventBeginPlay)

(event Collision|EventActorBeginOverlap
  (params (OtherActor :type Actor%20Object%20Reference)))

(event EventTick
  (params (DeltaSeconds :type Float%20%28single-precision%29)))

(event EventInteractwith
  (params (PlayerC :type BP%20First%20Person%20Character%20Object%20Reference))
  (bind _door_piv (Variables|Default|GetDoor_PIV))
  (bind _returnvalue (Transformation|GetWorldLocation _door_piv))
  (if (not (Variables|Default|GetIsRotating))
    (if (Variables|Default|GetdoorOpen)
      (Variables|Default|SetdoorOpen false)
      (bind _newtrack_0 (Timeline|T_DoorOpen ReverseFromEnd)
        (:Update
          (Variables|Default|SetIsRotating true)
          (Transformation|SetRelativeRotation (Variables|Default|GetDoor_PIV) (Math|Rotator|MakeRotator 0.0 0.0 (* _newtrack_0 -9e+01)) false false))
        (:Finished
          (Variables|Default|SetIsRotating false)))
      (else
        (bind _haskey (CallFunction|CheckKey PlayerC))
        (if _haskey
          (Audio|PlaySoundatLocation "/Engine/EditorSounds/GamePreview/EjectFromPlayer_Cue.EjectFromPlayer_Cue" _returnvalue "0, 0, 0" 1.0 1.0 0.0 0 0 0 0)
          (Variables|Default|SetdoorOpen true)
          (Timeline|T_DoorOpen PlayFromStart)
          (else
            (Audio|PlaySoundatLocation "/Engine/EditorSounds/Notifications/CompileFailed_Cue.CompileFailed_Cue" _returnvalue "0, 0, 0" 1.0 1.0 0.0 0 0 0 0)))))))

(fn ConstructionScript)

(fn CheckKey
  (params (Player%20C :type BP%20First%20Person%20Character%20Object%20Reference))
  (bind _inventorysystem (Variables|/Game/FirstPerson/Blueprints/BP_FirstPersonCharacter.BP_FirstPersonCharacter_C|GetInventorySystem Player%20C))
  (Variables|Default|SetHasKey false)
  (LocalVariables|SetLOCAL_InvRef _inventorysystem)
  (for _array_element (Variables|/Game/Blueprints/Inventory/InventorySystem.InventorySystem_C|GetContent _inventorysystem)
    (if (== (.id (Default|GetItemData (LocalVariables|GetLOCAL_InvRef) (.itemid _array_element))) (Variables|Default|GetKey))
      (Variables|Default|SetHasKey true)))
  (return (Variables|Default|GetHasKey)))

(fn Lookat
  (bind _itemdatacomponent (Variables|Default|GetItemDataComponent))
  (bind _itemid (Variables|/Game/Blueprints/Inventory/ItemDataComponent.ItemDataComponent_C|GetItemID _itemdatacomponent))
  (bind _returnvalue (Utilities|GetDataTableRow (.datatable _itemid) (.rowname _itemid))
    (:then
      (return (Utilities|Text|FormatText "Open {item}" (.Name (Utilities|Struct|BreakFItemStruct _returnvalue)))))))