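; BP_LootBag is a loot bag actor that holds items in an InventorySystem component and removes itself once it is empty.
; On each inventory update it checks whether the inventory is empty.
; If so, it casts player controller 0 to EscapeController, hides the container view on that HUD, then destroys itself.
; A failed cast leaves the bag in place.
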(event OnInventoryUpdate(InventorySystem)
  (if (Default|IsEmpty (Variables|Default|GetInventorySystem))
    (bind _asescape_controller (Utilities|Casting|CastToEscapeController (Game|GetPlayerController 0)))
    (Default|HideContainer (Variables|/Game/FirstPerson/Blueprints/EscapeController.EscapeController_C|GetHUD _asescape_controller))
    (Actor|DestroyActor)))

(event EventBeginPlay
  (|CallParentFunction) ; This node is disabled and will not be called.\nDrag off pins to build functionality.
)

(event Collision|EventActorBeginOverlap
  (params (OtherActor :type Actor%20Object%20Reference))
  (|CallParentFunction OtherActor) ; This node is disabled and will not be called.\nDrag off pins to build functionality.
)

(event EventTick
  (params (DeltaSeconds :type Float%20%28single-precision%29))
  (|CallParentFunction DeltaSeconds) ; This node is disabled and will not be called.\nDrag off pins to build functionality.
)

(fn ConstructionScript
  (|CallParentFunction))