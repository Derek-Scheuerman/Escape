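; Base Blueprint for items the player can pick up, carry and drop, showing an interact prompt on the HUD when looked at.
; Interacting with empty hands attaches the item to the player's ItemGrip, turns off physics and collision, and sets it as HeldItem.
; DropItem detaches it, places it at a short camera-forward trace hit or the trace end, then restores physics, collision and visibility.
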(event EventBeginPlay)

(event Collision|EventActorBeginOverlap
  (params (OtherActor :type Actor%20Object%20Reference)))

(event EventTick
  (params (DeltaSeconds :type Float%20%28single-precision%29)))

(event EventInteractwith
  (params (PlayerC :type BP%20First%20Person%20Character%20Object%20Reference))
  (bind _output_get (Variables|Default|SetPlayer%20C PlayerC))
  (Utilities|IsValid (Variables|/Game/FirstPerson/Blueprints/BP_FirstPersonCharacter.BP_FirstPersonCharacter_C|GetHeldItem _output_get)
    (:Is%20Not%20Valid
      (CallFunction|Pickup))))

(event EventLookat
  (params (PlayerC :type BP%20First%20Person%20Character%20Object%20Reference))
  (Widget|SetVisibility (Variables|/Game/Widgets/W_Hud.W_Hud_C|GetE_Interact (Variables|/Game/FirstPerson/Blueprints/BP_FirstPersonCharacter.BP_FirstPersonCharacter_C|GetHud PlayerC)) "Visible"))

(fn ConstructionScript)

(fn Pickup
  (bind _staticmesh (Variables|Default|GetStaticMesh))
  (Transformation|AttachComponentToComponent (Variables|/Game/FirstPerson/Blueprints/BP_FirstPersonCharacter.BP_FirstPersonCharacter_C|GetItemGrip (Variables|Default|GetPlayer%20C)) "None" "SnapToTarget" "KeepWorld" "KeepRelative" true)
  (Physics|SetSimulatePhysics _staticmesh false)
  (Collision|SetCollisionEnabled _staticmesh "NoCollision")
  (Variables|/Game/FirstPerson/Blueprints/BP_FirstPersonCharacter.BP_FirstPersonCharacter_C|SetHeldItem (Variables|Default|GetPlayer%20C) self))

(fn DropItem
  (bind _returnvalue (Game|GetPlayerCameraManager 0))
  (bind _staticmesh (Variables|Default|GetStaticMesh))
  (bind _returnvalue_2 (Camera|GetCameraLocation _returnvalue))
  (Transformation|DetachFromActor "KeepWorld" "KeepWorld" "KeepWorld")
  (bind _outhit (Collision|LineTraceByChannel _returnvalue_2 (+ _returnvalue_2 (* (Math|Vector|GetForwardVector (Camera|GetCameraRotation _returnvalue)) 2e+02)) "TraceTypeQuery1" false 0 "None"))
  (Transformation|SetActorLocation (Math|Vector|SelectVector (.Location (Collision|BreakHitResult _outhit)) (.TraceEnd (Collision|BreakHitResult _outhit)) (.bBlockingHit (Collision|BreakHitResult _outhit))) false false)
  (Physics|SetSimulatePhysics _staticmesh true)
  (Collision|SetCollisionEnabled _staticmesh "QueryAndPhysics")
  (Rendering|SetVisibility _staticmesh true false))